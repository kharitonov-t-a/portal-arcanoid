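; BlockBP is a breakable block that takes hits from BallBP actors.
; Each hit from a ball increments a counter, and the block destroys itself once the count reaches MaxCountHit.
; If it survives the first hit, its cube mesh switches to BasicShapeMaterial to show the damage.
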(event EventBeginPlay)

(event Collision|EventActorBeginOverlap
  (params (OtherActor :type Actor%20Object%20Reference)))

(event EventTick
  (params (DeltaSeconds :type Float%20%28single-precision%29)))

(event Collision|EventHit
  (params (MyComp :type Primitive%20Component%20Object%20Reference) (Other :type Actor%20Object%20Reference) (OtherComp :type Primitive%20Component%20Object%20Reference) (bSelfMoved :type Boolean) (HitLocation :type Vector :default "0, 0, 0") (HitNormal :type Vector :default "0, 0, 0") (NormalImpulse :type Vector :default "0, 0, 0") (Hit :type Hit%20Result%20Structure%20%28by%20ref%29))
  (Utilities|Casting|CastToBallBP Other)
  (bind _output_get (Variables|Default|SetcountHit (+ (Variables|Default|GetcountHit) 1)))
  (if (>= _output_get (Variables|Default|GetmaxCountHit))
    (Actor|DestroyActor)
    (else
      (switch int _output_get
        (:1
          (Rendering|Material|SetMaterial (Variables|Default|GetCube) 0 "/Game/BasicShapeMaterial.BasicShapeMaterial"))))))

(fn ConstructionScript)