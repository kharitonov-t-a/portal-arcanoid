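; BallBP is a ball actor that moves at constant speed, bounces off surfaces in the XY plane and can travel through portal walls.
; Tick sweeps it along Direction and reflects on blocking hits, while hitting a PlayerPawn blends in that pawn's last direction.
; PortalWall events cache the outer portal location; hitting an inner portal teleports the ball there, negating or axis-swapping Direction based on both portals' coordinates.
; Overlapping a KillZVolume broadcasts BallDestroyed and destroys it.
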(event OnComponentBeginOverlap(Sphere)
  (params (OverlappedComponent :type Primitive%20Component%20Object%20Reference) (OtherActor :type Actor%20Object%20Reference) (OtherComp :type Primitive%20Component%20Object%20Reference) (OtherBodyIndex :type Integer) (bFromSweep :type Boolean) (SweepResult :type Hit%20Result%20Structure%20%28by%20ref%29))
  (Utilities|Casting|CastToKillZVolume OtherActor)
  (Default|CallBallDestroyed)
  (Actor|DestroyActor))

(event Custom|CreateNewOutterPortal
  (params (location :type Vector))
  (bind _output_get (Variables|Default|SetlocationOutterPortal location))
  (Development|PrintString (Utilities|String|ToString(Vector) _output_get)))

(event EventBeginPlay
  (Variables|Default|Setdirection (Transformation|GetActorForwardVector))
  (bind _outactors (Actor|GetAllActorsOfClass "/Game/PortalWall.PortalWall_C"))
  (for _array_element _outactors
    (bind _asportal_wall (Utilities|Casting|CastToPortalWall _array_element))
    (EventDispatchers|BindEventtoNewOutterPortal _asportal_wall (delegate Custom|CreateNewOutterPortal))))

(event Collision|EventActorBeginOverlap
  (params (OtherActor :type Actor%20Object%20Reference)))

(event EventTick
  (params (DeltaSeconds :type Float%20%28single-precision%29))
  (bind _sweephitresult (Transformation|AddActorWorldOffset (* (Variables|Default|Getdirection) (* DeltaSeconds (Variables|Default|Getspeed))) true))
  (if (.bBlockingHit (Collision|BreakHitResult _sweephitresult))
    (Variables|Default|Setdirection (Math|Vector|MakeVector (.X (Math|Vector|BreakVector (Math|Vector|GetReflectionVector (Variables|Default|Getdirection) (.Normal (Collision|BreakHitResult _sweephitresult))))) (.Y (Math|Vector|BreakVector (Math|Vector|GetReflectionVector (Variables|Default|Getdirection) (.Normal (Collision|BreakHitResult _sweephitresult))))) 0.0))))

(event Collision|EventHit
  (params (MyComp :type Primitive%20Component%20Object%20Reference) (Other :type Actor%20Object%20Reference) (OtherComp :type Primitive%20Component%20Object%20Reference) (bSelfMoved :type Boolean) (HitLocation :type Vector :default "0, 0, 0") (HitNormal :type Vector :default "0, 0, 0") (NormalImpulse :type Vector :default "0, 0, 0") (Hit :type Hit%20Result%20Structure%20%28by%20ref%29))
  (bind _locationoutterportal (Variables|Default|GetlocationOutterPortal))
  (Utilities|FlowControl|Sequence
    (:then_0
      (bind _asportal_wall (Utilities|Casting|CastToPortalWall Other))
      (if (Variables|/Game/PortalWall.PortalWall_C|GetisInnerPortal _asportal_wall)
        (if (not (Math|Vector|Equal(Vector) (Variables|Default|GetlocationOutterPortal) "6666.000000, 0, 0" 0.0001))
          (Development|PrintString "Hello")
          (Transformation|SetWorldLocation (Variables|Default|GetSphere) (Variables|Default|GetlocationOutterPortal) false false)
          (if (Math|Boolean|ORBoolean (== (.x _locationoutterportal) (.x (Transformation|GetWorldLocation (Variables|/Game/PortalWall.PortalWall_C|GetPortalPoint _asportal_wall)))) (== (.y _locationoutterportal) (.y (Transformation|GetWorldLocation (Variables|/Game/PortalWall.PortalWall_C|GetPortalPoint _asportal_wall)))) (== (Math|Float|Truncate (.x _locationoutterportal)) (Math|Float|Truncate (* (.x (Transformation|GetWorldLocation (Variables|/Game/PortalWall.PortalWall_C|GetPortalPoint _asportal_wall))) -1.0))) (== (Math|Float|Truncate (.y _locationoutterportal)) (Math|Float|Truncate (* (.y (Transformation|GetWorldLocation (Variables|/Game/PortalWall.PortalWall_C|GetPortalPoint _asportal_wall))) -1.0))))
            (Variables|Default|Setdirection (Math|Vector|NegateVector (Variables|Default|Getdirection)))
            (else
              (Variables|Default|Setdirection (Math|Vector|MakeVector (.y (Variables|Default|Getdirection)) (.x (Variables|Default|Getdirection)) 0.0)))))))
    (:then_1
      (bind _asplayer_pawn (Utilities|Casting|CastToPlayerPawn Other))
      (Variables|Default|Setdirection (Math|Vector|Normalize (+ (Math|Vector|Normalize (Variables|/Game/PlayerPawn.PlayerPawn_C|GetlastDirection _asplayer_pawn)) (Variables|Default|Getdirection)))))))

(fn ConstructionScript)